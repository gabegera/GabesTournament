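; AI controller for the sniper enemy that runs its behavior tree with the player pawn as focus and blackboard target.
; On begin play it also marks the enemy unarmed, and perception updates on the player set the CanSeeTarget key and print a debug message.
; While that key is true, Tick draws a thin red debug line from the muzzle to the player.
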(event `self.ReceiveBeginPlay`
  (`self.RunBehaviorTree` "/Game/Characters/Enemies/AI/BehaviorTree/BT_SniperEnemy.BT_SniperEnemy")
  (`self.K2_SetFocus` (`GameplayStatics.GetPlayerPawn` 0))
  (`BlackboardComponent.SetValueAsObject` (`AIBlueprintHelperLibrary.GetBlackboard` null) "Target" (`GameplayStatics.GetPlayerPawn` 0))
  (`BlackboardComponent.SetValueAsBool` (`AIBlueprintHelperLibrary.GetBlackboard` null) "IsArmed" false))

(event `self.PerceptionComponent.OnTargetPerceptionUpdated`
  (params (Actor :type "Actor Object Reference") (Stimulus :type "AIStimulus Structure"))
  (if (== Actor (`GameplayStatics.GetPlayerPawn` 0))
    (`BlackboardComponent.SetValueAsBool` (`AIBlueprintHelperLibrary.GetBlackboard` null) "CanSeeTarget" Stimulus_bSuccessfullySensed)
    (`KismetSystemLibrary.PrintString` "Hello")))

(event `self.ReceiveTick`
  (params (DeltaSeconds :type "Float (single-precision)"))
  (if (`BlackboardComponent.GetValueAsBool` (`AIBlueprintHelperLibrary.GetBlackboard` null) "CanSeeTarget")
    (`KismetSystemLibrary.DrawDebugLine` (`self.GetMuzzleLocation`) (`self.K2_GetActorLocation` (`GameplayStatics.GetPlayerPawn` 0)) (struct :`R` 1.0 :`A` 1.0) 0.03 1.0)))

(fn `UserConstructionScript`)