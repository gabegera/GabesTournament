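; Player controller for the shooter character that routes Enhanced Input actions to shoot, look, move, dash, crouch, jump and weapon-slot handling.
; Most actions call functions not defined in this graph, while nine slot actions call EquipWeapon on the player character.
; Dash waits for cooldown, using the action's Z as a pressed flag and XY as direction for the character's dash timeline.
; Pickup only resets the HUD item name; aiming is stubbed.
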(event Input|EnhancedActionEvents|EnhancedInputActionIA_Jump
  (params (ActionValue :type Boolean) (ElapsedSeconds :type Float%20%28double-precision%29) (TriggeredSeconds :type Float%20%28double-precision%29) (InputAction :type Input%20Action%20Object%20Reference :default "/Game/Input/Actions/IA_Jump.IA_Jump"))
  (Class|ShooterPlayerController|Jump))

(event Input|EnhancedActionEvents|EnhancedInputActionIA_Dash
  (params (ActionValue :type Vector :default "0, 0, 0") (ElapsedSeconds :type Float%20%28double-precision%29) (TriggeredSeconds :type Float%20%28double-precision%29) (InputAction :type Input%20Action%20Object%20Reference :default "/Game/Input/Actions/IA_Dash.IA_Dash"))
  (if (and (> (.z ActionValue) 0.0) (<= (Variables|Default|GetDashCooldownValue) 0.0))
    (bind _asbp_shooter_player_character (Utilities|Casting|CastToBP_ShooterPlayerCharacter (Variables|Default|GetPlayerCharacter)))
    (Default|UseDashTimeline _asbp_shooter_player_character (.x ActionValue) (.y ActionValue))
    (Class|ShooterPlayerController|Dash)))

(event Input|EnhancedActionEvents|EnhancedInputActionIA_EquipSlot2
  (params (ActionValue :type Boolean) (ElapsedSeconds :type Float%20%28double-precision%29) (TriggeredSeconds :type Float%20%28double-precision%29) (InputAction :type Input%20Action%20Object%20Reference :default "/Game/Input/Actions/IA_EquipSlot2.IA_EquipSlot2"))
  (Class|ShooterCharacter|EquipWeapon (Variables|Default|GetPlayerCharacter) "Slot2"))

(event Input|EnhancedActionEvents|EnhancedInputActionIA_EquipSlot3
  (params (ActionValue :type Boolean) (ElapsedSeconds :type Float%20%28double-precision%29) (TriggeredSeconds :type Float%20%28double-precision%29) (InputAction :type Input%20Action%20Object%20Reference :default "/Game/Input/Actions/IA_EquipSlot3.IA_EquipSlot3"))
  (Class|ShooterCharacter|EquipWeapon (Variables|Default|GetPlayerCharacter) "Slot3"))

(event Input|EnhancedActionEvents|EnhancedInputActionIA_EquipSlot4
  (params (ActionValue :type Boolean) (ElapsedSeconds :type Float%20%28double-precision%29) (TriggeredSeconds :type Float%20%28double-precision%29) (InputAction :type Input%20Action%20Object%20Reference :default "/Game/Input/Actions/IA_EquipSlot4.IA_EquipSlot4"))
  (Class|ShooterCharacter|EquipWeapon (Variables|Default|GetPlayerCharacter) "Slot4"))

(event Input|EnhancedActionEvents|EnhancedInputActionIA_Shoot
  (params (ActionValue :type Boolean) (ElapsedSeconds :type Float%20%28double-precision%29) (TriggeredSeconds :type Float%20%28double-precision%29) (InputAction :type Input%20Action%20Object%20Reference :default "/Game/Input/Actions/IA_Shoot.IA_Shoot"))
  ;[1 1 1] Shooting
  (Class|ShooterPlayerController|Shoot))

(event Input|EnhancedActionEvents|EnhancedInputActionIA_EquipSlot5
  (params (ActionValue :type Boolean) (ElapsedSeconds :type Float%20%28double-precision%29) (TriggeredSeconds :type Float%20%28double-precision%29) (InputAction :type Input%20Action%20Object%20Reference :default "/Game/Input/Actions/IA_EquipSlot5.IA_EquipSlot5"))
  (Class|ShooterCharacter|EquipWeapon (Variables|Default|GetPlayerCharacter) "Slot5"))

(event Input|EnhancedActionEvents|EnhancedInputActionIA_EquipSlot6
  (params (ActionValue :type Boolean) (ElapsedSeconds :type Float%20%28double-precision%29) (TriggeredSeconds :type Float%20%28double-precision%29) (InputAction :type Input%20Action%20Object%20Reference :default "/Game/Input/Actions/IA_EquipSlot6.IA_EquipSlot6"))
  (Class|ShooterCharacter|EquipWeapon (Variables|Default|GetPlayerCharacter) "Slot6"))

(event Input|EnhancedActionEvents|EnhancedInputActionIA_EquipSlot7
  (params (ActionValue :type Boolean) (ElapsedSeconds :type Float%20%28double-precision%29) (TriggeredSeconds :type Float%20%28double-precision%29) (InputAction :type Input%20Action%20Object%20Reference :default "/Game/Input/Actions/IA_EquipSlot7.IA_EquipSlot7"))
  (Class|ShooterCharacter|EquipWeapon (Variables|Default|GetPlayerCharacter) "Slot7"))

(event Input|EnhancedActionEvents|EnhancedInputActionIA_EquipSlot8
  (params (ActionValue :type Boolean) (ElapsedSeconds :type Float%20%28double-precision%29) (TriggeredSeconds :type Float%20%28double-precision%29) (InputAction :type Input%20Action%20Object%20Reference :default "/Game/Input/Actions/IA_EquipSlot8.IA_EquipSlot8"))
  (Class|ShooterCharacter|EquipWeapon (Variables|Default|GetPlayerCharacter) "Slot8"))

(event Input|EnhancedActionEvents|EnhancedInputActionIA_EquipSlot9
  (params (ActionValue :type Boolean) (ElapsedSeconds :type Float%20%28double-precision%29) (TriggeredSeconds :type Float%20%28double-precision%29) (InputAction :type Input%20Action%20Object%20Reference :default "/Game/Input/Actions/IA_EquipSlot9.IA_EquipSlot9"))
  (Class|ShooterCharacter|EquipWeapon (Variables|Default|GetPlayerCharacter) "Slot9"))

(event Input|EnhancedActionEvents|EnhancedInputActionIA_Crouch
  (params (ActionValue :type Boolean) (ElapsedSeconds :type Float%20%28double-precision%29) (TriggeredSeconds :type Float%20%28double-precision%29) (InputAction :type Input%20Action%20Object%20Reference :default "/Game/Input/Actions/IA_Crouch.IA_Crouch"))
  (:Triggered
    (Class|ShooterPlayerController|Crouch))
  (:Completed
    (Class|ShooterPlayerController|StopCrouch)))

(event Input|EnhancedActionEvents|EnhancedInputActionIA_EquipSlot1
  (params (ActionValue :type Boolean) (ElapsedSeconds :type Float%20%28double-precision%29) (TriggeredSeconds :type Float%20%28double-precision%29) (InputAction :type Input%20Action%20Object%20Reference :default "/Game/Input/Actions/IA_EquipSlot1.IA_EquipSlot1"))
  (Class|ShooterCharacter|EquipWeapon (Variables|Default|GetPlayerCharacter) "Slot1"))

(event Input|EnhancedActionEvents|EnhancedInputActionIA_Look
  (params (ActionValue :type Vector%202D%20Structure) (ElapsedSeconds :type Float%20%28double-precision%29) (TriggeredSeconds :type Float%20%28double-precision%29) (InputAction :type Input%20Action%20Object%20Reference :default "/Game/Input/Actions/IA_Look.IA_Look"))
  (Class|ShooterPlayerController|AddLookInput ActionValue))

(event Input|EnhancedActionEvents|EnhancedInputActionIA_Move
  (params (ActionValue :type Vector%202D%20Structure) (ElapsedSeconds :type Float%20%28double-precision%29) (TriggeredSeconds :type Float%20%28double-precision%29) (InputAction :type Input%20Action%20Object%20Reference :default "/Game/Input/Actions/IA_Move.IA_Move"))
  (Class|ShooterPlayerController|Move (.x ActionValue) (.y ActionValue)))

(event Input|EnhancedActionEvents|EnhancedInputActionIA_PickupItem
  (params (ActionValue :type Boolean) (ElapsedSeconds :type Float%20%28double-precision%29) (TriggeredSeconds :type Float%20%28double-precision%29) (InputAction :type Input%20Action%20Object%20Reference :default "/Game/Input/Actions/IA_PickupItem.IA_PickupItem"))
  (bind _foundwidgets (Widget|GetAllWidgetsOfClass "/Game/Blueprints/Widgets/BPW_PlayerHUD.BPW_PlayerHUD_C" true))
  (for _array_element _foundwidgets
    (Variables|/Game/Blueprints/Widgets/BPW_PlayerHUD.BPW_PlayerHUD_C|SetPickupItemName _array_element "None")))

(event Input|EnhancedActionEvents|EnhancedInputActionIA_Aim
  (params (ActionValue :type Boolean) (ElapsedSeconds :type Float%20%28double-precision%29) (TriggeredSeconds :type Float%20%28double-precision%29) (InputAction :type Input%20Action%20Object%20Reference :default "/Game/Input/Actions/IA_Aim.IA_Aim")))

(event EventBeginPlay
  (Class|PlayerController|SetDeprecatedInputYawScale 1.0)
  (Class|PlayerController|SetDeprecatedInputPitchScale 1.0))

(event Input|KeyboardEvents|DebugKeyJ
  (params (Key :type Key%20Structure :default "None") (ActionValue :type Input%20Action%20Value%20Structure))
  (:Pressed
    (Class|PlayerController|AddYawInput 9e+01)))

(fn ConstructionScript)